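; BP_TVScreen is an interactable TV that cycles through screen images when the player presses E nearby.
; On BeginPlay it creates a hidden prompt widget, enables input, and applies a dynamic material instance showing the first texture.
; InteractBox overlaps with the third-person character toggle interaction and prompt visibility.
; Each valid press advances a wrapping index into the ScreenTexture array and updates the material's texture parameter.
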(event `self.ReceiveBeginPlay`
  (bind _returnvalue (`|CreateWidget` "/Game/UI/WBP_TVInteractPrompt.WBP_TVInteractPrompt_C" (`GameplayStatics.GetPlayerController` 0)))
  (bind _output_get (set `self.PromptWidget` _returnvalue))
  (`UserWidget.AddToViewport` _output_get 0)
  (`Widget.SetVisibility` _output_get "Hidden")
  (`self.EnableInput` (`GameplayStatics.GetPlayerController` 0))
  (bind _returnvalue_2 (`PrimitiveComponent.CreateDynamicMaterialInstance` (`self.Screen`) 0 "/Game/Materials/TV/MI_TVScreen_Dynamic.MI_TVScreen_Dynamic" "None"))
  (bind _output_get_2 (set `self.ScreenMID` _returnvalue_2))
  (`MaterialInstanceDynamic.SetTextureParameterValue` _output_get_2 "ScreenTexture" (`|GetArrayItem` (`self.ScreenTexture`))))

(event `Key|E`
  (params (Key :type "Key Structure"))
  (bind _screentexture (`self.ScreenTexture`))
  (:`Pressed`
    (if (`self.CanInteract`)
      (bind _output_get (set `self.CurrentTextureIndex` (mod (+ (`self.CurrentTextureIndex`) 1) (`KismetArrayLibrary.Array_Length` _screentexture))))
      (`MaterialInstanceDynamic.SetTextureParameterValue` (`self.ScreenMID`) "ScreenTexture" (`|GetArrayItem` _screentexture _output_get)))))

(event `self.InteractBox.OnComponentBeginOverlap`
  (params (OverlappedComponent :type "PrimitiveComponent Object Reference") (OtherActor :type "Actor Object Reference") (OtherComp :type "PrimitiveComponent Object Reference") (OtherBodyIndex :type Integer) (bFromSweep :type Boolean) (SweepResult :type "HitResult Structure (by ref)"))
  ; Can interact
  (cast `/Game/ThirdPerson/Blueprints/BP_ThirdPersonCharacter` OtherActor)
  (set `self.CanInteract` true)
  (`Widget.SetVisibility` (`self.PromptWidget`) "Visible"))

(event `self.InteractBox.OnComponentEndOverlap`
  (params (OverlappedComponent :type "PrimitiveComponent Object Reference") (OtherActor :type "Actor Object Reference") (OtherComp :type "PrimitiveComponent Object Reference") (OtherBodyIndex :type Integer))
  ; Can not interact
  (cast `/Game/ThirdPerson/Blueprints/BP_ThirdPersonCharacter` OtherActor)
  (set `self.CanInteract` false)
  (`Widget.SetVisibility` (`self.PromptWidget`) "Hidden"))

(fn `UserConstructionScript`)